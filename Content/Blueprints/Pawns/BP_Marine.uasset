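; BP_Marine is a player pawn with twin-stick style controls: movement along world X and Y axes, with aim set independently through controller yaw.
; Any key press records whether a gamepad is active, and Tick picks thumbstick or mouse aiming accordingly.
; Both modes ignore input inside a deadzone and derive yaw via atan2.
; Mouse aim follows the direction of mouse velocity rather than cursor position, smoothed with RInterpTo, while thumbstick aim snaps directly.
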(event EventBeginPlay)

(event Collision|EventActorBeginOverlap
  (params (OtherActor :type Actor%20Object%20Reference)))

(event EventTick
  (params (DeltaSeconds :type Float%20%28single-precision%29))
  (CallFunction|UdpatePlayerAim))

(event Input|AxisEvents|InputAxisMoveForward
  (params (AxisValue :type Float%20%28single-precision%29))
  (Pawn|Input|AddMovementInput "1.000000, 0, 0" AxisValue false))

(event Input|AxisEvents|InputAxisMoveRight
  (params (AxisValue :type Float%20%28single-precision%29))
  (Pawn|Input|AddMovementInput "0.000000,1.000000, 0" AxisValue false))

(event Input|KeyboardEvents|AnyKey
  (params (Key :type Key%20Structure :default "None"))
  (:Pressed
    (Variables|Default|SetGamepad%20Active (Class|KismetInputLibrary|KeyIsGamepadKey Key))))

(fn ConstructionScript)

(fn UdpatePlayerAim
  (if (Variables|Default|GetGamepad%20Active)
    (Thumbstickinput|UpdateThumbstickAim)
    (else
      (MouseInput|UpdateMouseAim))))

(fn IsThumbstickAboveDeadzone
  (return (> (Math|Vector2D|Vector2DLength (Math|Vector2D|MakeVector2D (Input|AxisValues|GetThumbstickAimUp) (Input|AxisValues|GetThumbstickAimRight))) (Variables|Thumbstickinput|GetThumbstick%20Deadzone))))

(fn GetMouseVelocity
  (bind _returnvalue (Game|GetPlayerController 0))
  (bind (_deltax _deltay) (Class|PlayerController|GetInputMouseDelta _returnvalue))
  (return (/ (Math|Vector2D|MakeVector2D _deltax _deltay) (Utilities|Time|GetWorldDeltaSeconds))))

(fn IsMouseAboveDeadzone
  (return (> (Math|Vector2D|Vector2DLength (MouseInput|GetMouseVelocity)) (Variables|Thumbstickinput|GetMouse%20Deadzone))))

(fn UpdateMouseAim
  (if (MouseInput|IsMouseAboveDeadzone)
    (Pawn|SetControlRotation (Game|GetPlayerController 0) (MouseInput|GetMouseAimDirection))))

(fn GetMouseAimDirection
  (bind _returnvalue (MouseInput|GetMouseVelocity))
  (return (Math|Interpolation|RInterpTo (Pawn|GetControlRotation (Game|GetPlayerController 0) :!class /Script/Engine.Controller) (Math|Rotator|MakeRotator 0.0 0.0 (Class|KismetMathLibrary|DegAtan2 (.x _returnvalue) (.y _returnvalue))) (Utilities|Time|GetWorldDeltaSeconds) (Variables|MouseInput|GetMouse%20Smoothing%20Strenght))))

(fn UpdateThumbstickAim
  (if (Thumbstickinput|IsThumbstickAboveDeadzone)
    (Pawn|SetControlRotation (Game|GetPlayerController 0) (Math|Rotator|MakeRotator 0.0 0.0 (Class|KismetMathLibrary|DegAtan2 (Input|AxisValues|GetThumbstickAimUp) (Input|AxisValues|GetThumbstickAimRight))))))