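; BP_SpawnMiniBoss is a spawner that creates BP_MiniBoss AI pawns at random points inside its Box volume.
; On BeginPlay it gathers existing mini-bosses once and, if their count is below SpawnAmount, waits SpawnTime, spawns one and prints a red on-screen message.
; It loops back to the count check without refreshing the actor list, so once started, spawning repeats without the cap taking effect.
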(event EventBeginPlay
  (bind _box (Variables|Default|GetBox))
  ;[1 0.6856 0] Spawn System Boss
  (bind _outactors (Actor|GetAllActorsOfClass "/Game/Blueprints/AI/BP_MiniBoss.BP_MiniBoss_C"))
  (if (< (Utilities|Array|Length _outactors) (Variables|Default|GetSpawn%20Amount)) :!label _label
    (Utilities|FlowControl|Delay (Variables|Default|GetSpawn%20Time))
    (AI|SpawnAIFromClass "/Game/Blueprints/AI/BP_MiniBoss.BP_MiniBoss_C" 0 (Math|Random|RandomPointinBoundingBox (Transformation|GetWorldLocation _box) (Components|Box|GetScaledBoxExtent _box)) "0, 0, 0" false 0)
    (Development|PrintString "BOSS SPAWNED" true true "(R=1.000000,G=0.000000,B=0.000000,A=1.000000)" 5.0)
    (goto _label)))

(fn ConstructionScript)