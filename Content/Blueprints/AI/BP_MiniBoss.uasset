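; Mini-boss character that chases the player, attacks in melee and is destroyed when its health runs out.
; A looping AIMoveTo pursues the player, while Tick pauses movement to play an attack montage within range and resumes it on completion.
; Damage lowers Health through ClampAngle, an angle clamp used on a plain value.
; DamagePlayer applies per-hit damage but is not called within this Blueprint.
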(event EventPossessed
  (params (NewController :type Controller%20Object%20Reference))
  (AI|AIMoveTo self "0, 0, 0" (Game|GetPlayerCharacter 0) 5.0 false :!label _label
    (:OnSuccess
      _)
    (:OnFail
      _))
  (Utilities|FlowControl|Delay 0.2)
  (goto _label))

(event EventTick
  (params (DeltaSeconds :type Float%20%28single-precision%29))
  (if (and (CallFunction|IsWithinAttackRange) (not (CallFunction|IsAttacking)))
    (CallFunction|DeactivateAIMovement)
    (Animation|Montage|PlayMontage (Variables|Character|GetMesh) "/Game/MiniBoss/Animations/MiniBossAttack2.MiniBossAttack2"
      (:OnCompleted
        (CallFunction|ActivateAIMovement)))))

(event Game|Damage|EventAnyDamage
  (params (Damage :type Float%20%28single-precision%29) (DamageType :type Damage%20Type%20Object%20Reference) (InstigatedBy :type Controller%20Object%20Reference) (DamageCauser :type Actor%20Object%20Reference))
  (bind _health (CallFunction|DeacreaseHealth Damage))
  (if (== _health 0.0)
    (Actor|DestroyActor)
    (Development|PrintString "BOSS KILLED" true true "(R=0.000000,G=0.660000,B=1.000000,A=1.000000)" 5.0)))

(fn ConstructionScript)

(fn IsWithinAttackRange
  (return (< (Transformation|GetDistanceTo (Game|GetPlayerCharacter 0)) (Variables|Default|GetAttack%20Range))))

(fn IsAttacking
  (return (Animation|Montage|MontageIsPlaying (Components|SkeletalMesh|GetAnimInstance (Variables|Character|GetMesh)) "/Game/MiniBoss/Animations/MiniBossAttack2.MiniBossAttack2")))

(fn DeactivateAIMovement
  (Components|Activation|Deactivate (Variables|Character|GetCharacterMovement)))

(fn ActivateAIMovement
  (Components|Activation|Activate (Variables|Character|GetCharacterMovement) false))

(fn DamagePlayer
  (Game|Damage|ApplyDamage (Game|GetPlayerCharacter 0) (Variables|Default|GetDamage%20Per%20Hit) 0 0))

(fn DeacreaseHealth
  (params (Damage%20Amount :type Float%20%28single-precision%29))
  (bind _output_get (Variables|Default|SetHealth%20 (Math|Float|ClampAngle (- (Variables|Default|GetHealth%20) Damage%20Amount) 0.0 (Variables|Default|GetHealth%20))))
  (return _output_get))